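; BP_FallTrigger01 is a fall trigger actor that restarts the current level when an overlap with its Box component ends.
; On BeginPlay it fades player 0's camera in from black over two seconds.
; When anything leaves the box, it fades the camera out, waits for the fade to finish, then reopens the current level by name.
; The end-overlap event does not filter which actor left.
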(event `self.ReceiveBeginPlay`
  (`PlayerCameraManager.StartCameraFade` (`PlayerController.PlayerCameraManager` (`GameplayStatics.GetPlayerController` 0)) 1.0 0.0 2.0 (struct :`A` 1.0) false false))

(event `self.Box.OnComponentEndOverlap`
  (params (OverlappedComponent :type "PrimitiveComponent Object Reference") (OtherActor :type "Actor Object Reference") (OtherComp :type "PrimitiveComponent Object Reference") (OtherBodyIndex :type Integer))
  (bind _returnvalue (`GameplayStatics.GetCurrentLevelName` true))
  (`PlayerCameraManager.StartCameraFade` :`self` (`PlayerController.PlayerCameraManager` (`GameplayStatics.GetPlayerController` 0)) :`FromAlpha` 0.0 :`ToAlpha` 1.0 :`Duration` 2.0)
  (`KismetSystemLibrary.Delay` 2.0)
  (`GameplayStatics.OpenLevel` (`KismetStringLibrary.Conv_StringToName` _returnvalue)))

(fn `UserConstructionScript`)